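; BP_Result is a target actor that receives item props, with its static mesh components acting as slots matched by mesh asset.
; ShowHighlight swaps materials on the component matching a prop, caching it as HighlightPart to revert on the next call or when switched off.
; SetItem applies a third material to the first matching component and destroys the prop.
; Slot state exists only as materials, with no filled-slot tracking.
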(fn `SetItem`
  (params (ItemProp :type "/Game/StaticMesh/BP_ItemProp Object Reference"))
  (for _array_element (`self.K2_GetComponentsByClass` "/Script/Engine.StaticMeshComponent")
    (if (== (`StaticMeshComponent.StaticMesh` _array_element) (`StaticMeshComponent.StaticMesh` (`/Game/StaticMesh/BP_ItemProp.StaticMesh` ItemProp)))
      (`PrimitiveComponent.SetMaterial` _array_element 0 "/Engine/VREditor/BasicMeshes/MI_Cube_03.MI_Cube_03")
      (`self.K2_DestroyActor` (`local.ItemProp`))
      (return))))

(fn `ShowHighlight`
  (params (ItemProp :type "/Game/StaticMesh/BP_ItemProp Object Reference") (IsOn :type Boolean))
  (if IsOn
    (`|ExecutionSequence`
      (:`then_0`
        (bind _highlightpart (`self.HighlightPart`)
          (:`then`
            (`PrimitiveComponent.SetMaterial` _highlightpart 0 "/Engine/VREditor/BasicMeshes/MI_Cube_02.MI_Cube_02"))
          (:`else`)))
      (:`then_1`
        (for _array_element (`self.K2_GetComponentsByClass` "/Script/Engine.StaticMeshComponent")
          (if (== (`StaticMeshComponent.StaticMesh` _array_element) (`StaticMeshComponent.StaticMesh` (`/Game/StaticMesh/BP_ItemProp.StaticMesh` ItemProp)))
            (bind _output_get (set `self.HighlightPart` _array_element))
            (`PrimitiveComponent.SetMaterial` _output_get 0 "/Engine/VREditor/BasicMeshes/MI_Cube_01.MI_Cube_01")))))
    (else
      (bind _highlightpart_2 (`self.HighlightPart`)
        (:`then`
          (`PrimitiveComponent.SetMaterial` _highlightpart_2 0 "/Engine/VREditor/BasicMeshes/MI_Cube_02.MI_Cube_02"))
        (:`else`)))))

(fn `UserConstructionScript`)