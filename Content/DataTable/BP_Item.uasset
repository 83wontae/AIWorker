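; BP_Item is an item actor that takes its static mesh from a row of the DT_Food data table, selected by RowName.
; The construction script applies that row's mesh, or a Cube when the row is not found.
; On BeginPlay, an item whose RowName is None picks a random row from the table and switches to its mesh.
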(event `self.ReceiveBeginPlay`
  (if (== (`self.RowName`) "None")
    (bind _outrownames (`DataTableFunctionLibrary.GetDataTableRowNames` "/Game/DataTable/DT_Food.DT_Food"))
    (bind _output_get (set `self.RowName` (`KismetArrayLibrary.Array_Random` _outrownames)))
    (bind _returnvalue (`|GetDataTableRow` "/Game/DataTable/DT_Food.DT_Food" _output_get)
      (:`then`
        (`StaticMeshComponent.SetStaticMesh` (`self.StaticMesh`) (`.StaticMesh_5_711BCFB54608D6CADA9398844F31893B` (break `/Game/DataTable/ST_Food` _returnvalue)))))))

(fn `UserConstructionScript`
  (bind _returnvalue (`|GetDataTableRow` "/Game/DataTable/DT_Food.DT_Food" (`self.RowName`))
    (:`then`
      (`StaticMeshComponent.SetStaticMesh` (`self.StaticMesh`) (`.StaticMesh_5_711BCFB54608D6CADA9398844F31893B` (break `/Game/DataTable/ST_Food` _returnvalue))))
    (:`RowNotFound`
      (`StaticMeshComponent.SetStaticMesh` (`self.StaticMesh`) "/Engine/BasicShapes/Cube.Cube"))))